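; Demo level switcher for a CAVE VR setup that opens one of three uvr levels from wand button presses.
; Tick polls UvrWasButtonPressed on the VRPN "WandButtons" device in two sequenced branch chains, each calling OpenLevelByName on a match.
; The first chain reads keyboard-bound channels that simulate the wand, while the second reads the real CAVE wand's channels.
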(event `self.ReceiveTick`
  (params (DeltaSeconds :type "Float (single-precision)"))
  (`|ExecutionSequence`
    (:`then_0`
      ;[1 1 1] VRPN-keyboard bindings for wand simulation
      (bind _returnvalue (`UVRBlueprintLibInput.UvrWasButtonPressed` "WandButtons" 79))
      (if _returnvalue
        (`GameplayStatics.OpenLevel` "uvr_level_1")
        (else
          (bind _returnvalue_2 (`UVRBlueprintLibInput.UvrWasButtonPressed` "WandButtons" 80))
          (if _returnvalue_2
            (`GameplayStatics.OpenLevel` "uvr_level_2")
            (else
              (bind _returnvalue_3 (`UVRBlueprintLibInput.UvrWasButtonPressed` "WandButtons" 81))
              (if _returnvalue_3
                (`GameplayStatics.OpenLevel` "uvr_level_3")))))))
    (:`then_1`
      ;[1 1 1] VRPN-wand bindings for real CAVE
      (bind _returnvalue_4 (`UVRBlueprintLibInput.UvrWasButtonPressed` "WandButtons" 1))
      (if _returnvalue_4
        (`GameplayStatics.OpenLevel` "uvr_level_1")
        (else
          (bind _returnvalue_5 (`UVRBlueprintLibInput.UvrWasButtonPressed` "WandButtons"))
          (if _returnvalue_5
            (`GameplayStatics.OpenLevel` "uvr_level_2")
            (else
              (bind _returnvalue_6 (`UVRBlueprintLibInput.UvrWasButtonPressed` "WandButtons" 2))
              (if _returnvalue_6
                (`GameplayStatics.OpenLevel` "uvr_level_3")))))))))

(fn `UserConstructionScript`)