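; Demo wand actor that binds itself to the UVR "wand" node and makes that node the translation direction source.
; On the first Tick it registers the translation direction ID and adds the UVR root as a tick prerequisite.
; Tick retries the node lookup until valid, then attaches to it and resets the scene root's relative transform, with boolean flags making each setup one-time.
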(event `self.ReceiveBeginPlay`
  ;[1 1 1] Attach wand implementation object to the wand node
  (set `self.InitializedTranslateDirection` false)
  (set `self.AttachedToUvrComponent` false))

(event `self.ReceiveTick`
  (params (DeltaSeconds :type "Float (single-precision)"))
  ;[1 1 1] Attach wand implementation object to the wand node
  (`|ExecutionSequence`
    (:`then_0`
      (if (not (`self.InitializedTranslateDirection`))
        (`UVRBlueprintLibGame.UvrSetTranslationDirectionComponentId` "wand")
        (bind _returnvalue (`UVRBlueprintLibGame.UvrGetRoot`))
        (`self.AddTickPrerequisiteActor` _returnvalue)
        (set `self.InitializedTranslateDirection` true)))
    (:`then_1`
      (if (not (`self.AttachedToUvrComponent`))
        (bind _returnvalue_2 (`UVRBlueprintLibGame.UvrGetNodeById` "wand"))
        (if (`KismetSystemLibrary.IsValid` _returnvalue_2)
          (`self.K2_AttachToComponent` _returnvalue_2 "None" "KeepRelative" "KeepRelative" "KeepRelative" false)
          (`SceneComponent.ResetRelativeTransform` (`self.DefaultSceneRoot1`))
          (set `self.AttachedToUvrComponent` true))))))

(fn `UserConstructionScript`)